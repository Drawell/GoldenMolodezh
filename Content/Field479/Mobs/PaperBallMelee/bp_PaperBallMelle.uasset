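; Paper ball melee enemy, a 2D flipbook mob with a health bar widget that it registers itself as owner of on BeginPlay.
; When PawnSensing spots a BaseChar, it runs AI MoveTo toward it, then returns to its spawn location whether the move succeeds or fails.
; An animation state implementation swaps the Paper flipbook between idle and walk.
; No attack logic is present; debug prints mark move results.
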(event OnSeePawn(PawnSensing)
  (params (Pawn :type Pawn%20Object%20Reference))
  (bind _asbase_char (Utilities|Casting|CastToBaseChar Pawn))
  (AI|AIMoveTo self "0, 0, 0" _asbase_char 5.0 false
    (:OnSuccess
      (Development|PrintString "succ"))
    (:OnFail
      (Development|PrintString "fail")))
  (AI|AIMoveTo self (Variables|Default|GetStartPosition) 0 5.0 false))

(event EventBeginPlay
  (bind _self self)
  (bind _asw_healt_bar (Utilities|Casting|CastTow_HealtBar (UserInterface|GetUserWidgetObject (Variables|Default|GetHealthWidget))))
  (Variables|/Game/Interface/Health/w_HealtBar.w_HealtBar_C|SetOwner _asw_healt_bar _self)
  (Variables|Default|SetStartPosition (Transformation|GetActorLocation _self)))

(event EventTick
  (params (DeltaSeconds :type Float%20%28single-precision%29)))

(event EventChangeAnimStateImplemetnation
  (params (NewAnimState :type EAnimStateEnum%20Enum :default "ASE_Idle"))
  (bind _paperflipbook (Variables|Default|GetPaperFlipbook))
  (switch Utilities|FlowControl|Switch|SwitchonEAnimStateEnum NewAnimState
    (:ASE_Idle
      (Sprite|SetFlipbook _paperflipbook "/Game/Field479/Mobs/PaperBallMelee/Sprites/fb_PaperBallM_idle1.fb_PaperBallM_idle1"))
    (:ASE_Run
      (Sprite|SetFlipbook _paperflipbook "/Game/Field479/Mobs/PaperBallMelee/Sprites/fb_PaperBallM_walk1.fb_PaperBallM_walk1"))))

(fn ConstructionScript)