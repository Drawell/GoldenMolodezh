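; Armor item Blueprint that represents the armor with four directional sprite components: Left, Right, Back and Front.
; On BeginPlay it adds each component to its matching per-direction component array, then calls ShowInWorld.
; The Construction Script is empty apart from a disconnected copy of that same setup, which never runs.
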(event EventBeginPlay
  (Utilities|Array|Add (Variables|Default|GetLeftComponents) (Variables|Default|GetLeft))
  (Utilities|Array|Add (Variables|Default|GetRightComponents) (Variables|Default|GetRight))
  (Utilities|Array|Add (Variables|Default|GetBackComponents) (Variables|Default|GetBack))
  (Utilities|Array|Add (Variables|Default|GetFrontComponents) (Variables|Default|GetFront))
  (Class|ArmorBase|ShowinWorld))

(event Collision|EventActorBeginOverlap
  (params (OtherActor :type Actor%20Object%20Reference)))

(event EventTick
  (params (DeltaSeconds :type Float%20%28single-precision%29)))

(fn ConstructionScript)